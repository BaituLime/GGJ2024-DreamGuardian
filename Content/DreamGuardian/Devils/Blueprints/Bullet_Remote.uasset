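; Bullet_Remote is a short-lived damage hitbox, apparently for a devil's ranged attack.
; On BeginPlay it sets its box's X extent to BoxLength, then destroys itself after a brief delay.
; Any overlapping Human loses sweet dream value and any CatCharacter loses health, both by AttackValue.
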(event `self.ReceiveBeginPlay`
  (bind _box (`self.Box`))
  (bind (_boxextent_x _boxextent_y _boxextent_z) (`KismetMathLibrary.BreakVector` (`BoxComponent.BoxExtent` _box)))
  (`BoxComponent.SetBoxExtent` _box (`KismetMathLibrary.MakeVector` (`self.BoxLength`) _boxextent_y _boxextent_z) true)
  (`KismetSystemLibrary.Delay` 0.2)
  (`self.K2_DestroyActor`))

(event `self.ReceiveActorBeginOverlap`
  (params (OtherActor :type "Actor Object Reference"))
  (bind _attackvalue (`self.AttackValue`))
  (bind _ashuman (cast `Human` OtherActor)
    (:`then`
      (`Human.DecreaseSweetDreamValue` _ashuman _attackvalue))
    (:`CastFailed`
      (bind _ascat_character (cast `CatCharacter` OtherActor))
      (`CatCharacter.DecreaseHealthValue` _ascat_character _attackvalue))))

(fn `UserConstructionScript`)