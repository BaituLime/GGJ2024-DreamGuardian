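; Devil_Flash is a devil that periodically attacks every Human around it, lowering their quiet value.
; Tick accumulates a timer and, once it passes the attack time, runs a debug-drawn multi sphere trace on the BlockAll profile at its own location, sized by its attack scope.
; Human hits receive DecreaseQuietValue with the attack value and a printed message.
; The separate Attack event only prints a message naming its target.
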(event `self.ReceiveTick`
  (params (DeltaSeconds :type "Float (single-precision)"))
  (bind _returnvalue (`self.K2_GetActorLocation`))
  (bind _output_get (set `self.AttackTimer` (+ (`self.AttackTimer`) DeltaSeconds)))
  (if (> _output_get (`self.AttackTime`))
    (set `self.AttackTimer` 0.0)
    (bind (_outhits _returnvalue_2) (`KismetSystemLibrary.SphereTraceMultiByProfile` _returnvalue _returnvalue (`self.GetAttackScope`) "BlockAll" false (`|MakeArray` self) "ForDuration"))
    (if _returnvalue_2
      (for _array_element _outhits
        (bind _ashuman (cast `Human` (`.HitActor` (`GameplayStatics.BreakHitResult` _array_element))))
        (`Human.DecreaseQuietValue` _ashuman (`self.GetAttackValue`))
        (`KismetSystemLibrary.PrintText` (`|FormatText` "DevilFlash Attacks {0}." (`KismetSystemLibrary.GetDisplayName` (`.HitActor` (`GameplayStatics.BreakHitResult` _array_element)))))))))

(event `self.Attack`
  (params (TargetActor :type "Actor Object Reference"))
  (`KismetSystemLibrary.PrintText` (`|FormatText` "DevilFlash Attacks {0}." (`KismetSystemLibrary.GetDisplayName` TargetActor))))

(fn `UserConstructionScript`)