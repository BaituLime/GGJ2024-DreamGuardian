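; Devil_Remote is a ranged devil enemy that attacks its target with Bullet_Remote projectiles.
; Attack stores the target and plays the AM_EnemyRemote montage, while a separate ActualAttack event prints a debug message and spawns the bullet.
; The bullet spawns one attack scope along the devil's forward vector, yawed toward the target, and receives the scope as box length plus the attack value.
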(event `self.ActualAttack`
  (bind _returnvalue (`self.K2_GetActorLocation`))
  (bind _returnvalue_2 (`self.GetAttackScope`))
  (bind _target_actor (`self.Target Actor`))
  (bind (_returnvalue_roll _returnvalue_pitch _returnvalue_yaw) (`KismetMathLibrary.BreakRotator` (`KismetMathLibrary.MakeRotFromX` (- (`self.K2_GetActorLocation` _target_actor) _returnvalue))))
  (`KismetSystemLibrary.PrintText` (`|FormatText` "DevilRemote Attacks {0}." (`KismetSystemLibrary.GetDisplayName` _target_actor)))
  (`|SpawnActorFromClass` "/Game/DreamGuardian/Devils/Blueprints/Bullet_Remote.Bullet_Remote_C" (`KismetMathLibrary.MakeTransform` (+ _returnvalue (* (`self.GetActorForwardVector`) _returnvalue_2)) (`KismetMathLibrary.MakeRotator` 0.0 0.0 _returnvalue_yaw)) "AlwaysSpawn" "MultiplyWithRoot" null _returnvalue_2 (`self.GetAttackValue`) null))

(event `self.Attack`
  (params (TargetActor :type "Actor Object Reference"))
  (set `self.Target Actor` TargetActor)
  (`|PlayMontage` (`self.Mesh`) "/Game/CharacterKIT/Animations/AM_EnemyRemote.AM_EnemyRemote"))

(fn `UserConstructionScript`)